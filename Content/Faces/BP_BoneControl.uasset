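; Face mask actor that mirrors RealSense head and facial tracking on a poseable skeletal mesh.
; Each tick applies head location, nudged toward a center point, and rotation, then moves landmark-ID-named bones.
; A delayed capture with countdown widget, triggered by input or manager, records per-landmark offsets from reset bone positions to correct tracking.
; Input cycles mask meshes and immediately recaptures offsets; the manager controls visibility.
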(event `InputAction|Next_Mask`
  (params (Key :type "Key Structure" :default "AnyKey"))
  ;[1 1 1] Mask switching
  (:`Pressed`
    (bind _output_get (set `self.MaskIndex` (+ (`self.MaskIndex`) 1)))
    (if (>= _output_get (`self.NumMasks`))
      (set `self.MaskIndex` 0))
    (`self.ChangeMask` (`self.MaskIndex`))))

(event `InputAction|Last_Mask`
  (params (Key :type "Key Structure" :default "AnyKey"))
  ;[1 1 1] Mask switching
  (:`Pressed`
    (bind _output_get (set `self.MaskIndex` (- (`self.MaskIndex`) 1)))
    (if (< _output_get 0)
      (set `self.MaskIndex` (- (`self.NumMasks`) 1)))
    (`self.ChangeMask` (`self.MaskIndex`))))

(event `InputAction|Capture_Relaxed_Pose`
  (params (Key :type "Key Structure" :default "AnyKey"))
  ;[1 1 1] Capture landmark offset when pressing ENTER
  (:`Pressed`
    (`self.InitCapture`)))

(event `self.ReceiveTick`
  (params (DeltaSeconds :type "Float (single-precision)"))
  (bind _poseablemesh (`self.PoseableMesh`))
  (bind _widget (`self.Widget`))
  (bind _manager (`self.Manager`))
  (bind _manager_2 (`self.Manager`))
  (bind _m_headlocation (`RealSenseActor.m_headLocation` _manager))
  (bind _newlocation (`self.FixHeadLocation` _m_headlocation))
  ;[1 1 1] Every frame
  (if (`self.CaptureAfterDelay`)
    (bind _output_get (set `self.TimeBeforeCapture` (- (`self.TimeBeforeCapture`) DeltaSeconds)))
    (bind _output_get_2 (set `/Game/Faces/WB_CaptureDelay.Delay` _output_get _widget))
    (if (<= _output_get_2 0.0)
      (set `self.CaptureAfterDelay` false)
      (set `/Game/Faces/WB_CaptureDelay.Show` false _widget)
      (`self.Capture Defaults`)))
  ;;[1 1 1] Handle RealSense events
  (if (`RealSenseActor.m_shouldCaptureDefault` _manager_2)
    (`self.InitCapture`))
  (`self.SetActorHiddenInGame` (`RealSenseActor.m_shouldMaskBeHidden` _manager_2))
  ;;[1 1 1] Update loc/rot every frame
  ;;;[1 1 1] Set Location and Rotation of actor
  (`self.K2_SetActorLocation` _newlocation)
  (`ActorUtilities.SetActorRotationQuat` self (`RealSenseActor.m_headRotation` _manager))
  ;;;[1 1 1] Set Location of all  bones
  (for _array_element (`RealSenseActor.m_landmarks` _manager)
    (bind (_location _identifier) (break `Landmark` _array_element))
    (bind _name (`self.IntToName` _identifier))
    (if (!= (`SkinnedMeshComponent.GetBoneIndex` _poseablemesh _name) -1)
      (if (`self.hasCapturedOffsets`)
        (bind _returnvalue (`RealSenseActor.getLandmarkById` (`self.Offset Landmarks`) _identifier))
        (`PoseableMeshComponent.SetBoneLocationByName` _poseablemesh _name (+ (- (+ (`.location` (break `Landmark` _returnvalue)) _location) _m_headlocation) _newlocation) "WorldSpace") ; set pose with offset
        (else
          (`PoseableMeshComponent.SetBoneLocationByName` _poseablemesh _name _location "WorldSpace") ; set pose without offset
        )))))

(event `self.ReceiveBeginPlay`
  ;[1 1 1] Get Realsense manager
  (bind _outactors (`GameplayStatics.GetAllActorsOfClass` "/Script/Anerops.RealSenseActor"))
  (set `self.Manager` (`KismetArrayLibrary.Array_Get` _outactors))
  ;[1 1 1] Create Delay widget
  (bind _returnvalue (`|CreateWidget` "/Game/Faces/WB_CaptureDelay.WB_CaptureDelay_C" null self))
  (bind _output_get (set `self.Widget` _returnvalue))
  (`UserWidget.AddToViewport` _output_get 0))

(event `self.ReceiveDestroyed`
  ;[1 1 1] Remove widget
  (`Widget.RemoveFromParent` (`self.Widget`)))

(fn `Capture Defaults`
  (bind _poseablemesh (`self.PoseableMesh`))
  (bind _m_headlocation (`RealSenseActor.m_headLocation` (`self.Manager`)))
  ;[1 1 1] Remove old values
  (`KismetArrayLibrary.Array_Clear` (`self.Offset Landmarks`))
  (for _array_element (`RealSenseActor.m_landmarks` (`self.Manager`))
    (bind (_location _identifier) (break `Landmark` _array_element))
    (bind _name (`self.IntToName` _identifier))
    (if (!= (`SkinnedMeshComponent.GetBoneIndex` _poseablemesh _name) -1)
      (`PoseableMeshComponent.ResetBoneTransformByName` _poseablemesh _name)
      (bind _returnvalue (`PoseableMeshComponent.GetBoneLocationByName` _poseablemesh _name "WorldSpace"))
      (`KismetArrayLibrary.Array_Add` (`self.Offset Landmarks`) (make `Landmark` (- (+ (- _returnvalue (`self.FixHeadLocation` _m_headlocation)) _m_headlocation) _location) _identifier)) ; Add after removing head fix
    ))
  (set `self.hasCapturedOffsets` true)
  (return))

(fn `ChangeMask`
  (params (Index :type Integer))
  (bind _poseablemesh (`self.PoseableMesh`))
  (switch `int` Index
    (:`Default`
      _)
    (:`0`
      (`SkinnedMeshComponent.SetSkinnedAssetAndUpdate` _poseablemesh "/Game/Faces/SK_Bob.SK_Bob" false)
      (`self.Capture Defaults` :!label _label))
    (:`1`
      (`SkinnedMeshComponent.SetSkinnedAssetAndUpdate` _poseablemesh "/Game/Faces/SK_Batman.SK_Batman" false)
      (goto _label))
    (:`2`
      (`SkinnedMeshComponent.SetSkinnedAssetAndUpdate` _poseablemesh "/Game/Faces/SK_Bob.SK_Bob" false)
      (goto _label))
    (:`3`
      (`SkinnedMeshComponent.SetSkinnedAssetAndUpdate` _poseablemesh "/Game/Faces/SK_Goblin.SK_Goblin" false)
      (goto _label)))
  (return))

(fn `FixHeadLocation`
  (params (Location :type "Vector Structure"))
  (returns (NewLocation :type "Vector Structure"))
  (return (`KismetMathLibrary.VLerp` (+ Location (`self.MaskOffset`)) (`self.Center`) (`self.CenterPush`))))

(fn `InitCapture`
  (set `RealSenseActor.m_shouldCaptureDefault` false (`self.Manager`))
  (set `self.CaptureAfterDelay` true)
  (set `/Game/Faces/WB_CaptureDelay.Show` true (`self.Widget`))
  (set `self.TimeBeforeCapture` (`self.CaptureDelay`)) ; Set the delay before capture
  (return))

(fn `IntToName`
  (params (Integer :type "Integer (by ref)"))
  (returns (Name :type Name))
  (return (`KismetStringLibrary.Conv_StringToName` (`KismetStringLibrary.Conv_IntToString` Integer))))

(fn `LogVector`
  (params (Vector :type "Vector Structure"))
  (`KismetSystemLibrary.PrintText` (`KismetTextLibrary.Conv_VectorToText` Vector) false true (struct :`G` 0.66 :`B` 1.0 :`A` 1.0) 0.0)
  (return))

(fn `UserConstructionScript`)